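; LuckyEnemyBP is an enemy pawn that moves continuously along its own forward vector through movement input applied every Tick.
; BeginPlay caches the first player pawn as its target, but no live logic uses it.
; An AIMoveTo chase toward that target, gated by a chasing flag, is left unconnected and never runs, so the enemy does not steer toward the player.
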(event EventBeginPlay
  (Variables|Default|SetmTarget (Game|Player|GetPlayerPawn 0)))

(event Collision|EventActorBeginOverlap
  (params (OtherActor :type Actor%20Object%20Reference)))

(event EventTick
  (params (DeltaSeconds :type Float%20%28single-precision%29))
  (Pawn|Input|AddMovementInput (Transformation|GetActorForwardVector) 1e+02 false))

(fn ConstructionScript)