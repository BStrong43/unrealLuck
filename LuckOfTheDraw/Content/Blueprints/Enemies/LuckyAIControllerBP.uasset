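; AI controller Blueprint for the Lucky enemy that makes it chase the player.
; On BeginPlay it snaps and attaches itself to its enemy actor.
; ActiveTick sets the player pawn as the destination, and OnPathingTick runs AIMoveTo on the enemy toward the stored target within a set acceptance radius.
; Move success and failure only print debug messages, and the standard Tick is unused.
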(event EventBeginPlay
  (Transformation|AttachActorToActor (Variables|Default|GetmEnemySelf) "None" "SnapToTarget" "SnapToTarget" "SnapToTarget" true))

(event EventTick
  (params (DeltaSeconds :type Float%20%28single-precision%29)))

(event EventActiveTick
  (params (DeltaTime :type Float%20%28single-precision%29))
  (Class|LuckyAIController|SetDesttoActor (Game|Player|GetPlayerPawn 0)))

(event EventOnPathingTick
  (bind _movementresult (AI|AIMoveTo (Variables|Default|GetmEnemySelf) (Variables|Default|GetmTarget) 0 (Variables|Default|GetmTermRadius) false)
    (:OnSuccess
      (Development|PrintString "Successful Path" true true "(R=1.000000,G=0.000000,B=0.029223,A=1.000000)" 2e+01))
    (:OnFail
      (Development|PrintText (Utilities|Text|ToText(String) (Utilities|String|EnumtoString _movementresult)) true true "(R=0.000000,G=1.000000,B=0.002892,A=1.000000)" 2e+01))))

(fn ConstructionScript)